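; Player pawn Blueprint that shows match-result UI: victory, defeat, other-player elimination notices and a scoreboard.
; OnReceive events create WBP_GameNotice with Spanish text, replacing the previous notice tracked in WidgetDeAvisoActual; victory appears after a short delay.
; Elimination notices store that reference on the first local player's controlled pawn rather than on self.
; The scoreboard event simply adds WBP_Scoreboard to the viewport.
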(event `self.OnReceiveWinUI`
  (bind _widgetdeavisoactual (`self.WidgetDeAvisoActual`))
  (`KismetSystemLibrary.Delay` 1.5)
  (`/Engine/EditorBlueprintResources/StandardMacros.IsValid` _widgetdeavisoactual
    (:`Is Valid`
      (`Widget.RemoveFromParent` _widgetdeavisoactual))
    (:`Is Not Valid`
      _))
  (bind _returnvalue (`|CreateWidget` "/Game/UI/WBP_GameNotice.WBP_GameNotice_C"))
  (`/Game/UI/WBP_GameNotice.SetNoticeMessage` _returnvalue "¡VICTORIA!")
  (`UserWidget.AddToViewport` _returnvalue 0)
  (set `self.WidgetDeAvisoActual` _returnvalue))

(event `self.OnReceiveLoseUI`
  (bind _widgetdeavisoactual (`self.WidgetDeAvisoActual`))
  (`/Engine/EditorBlueprintResources/StandardMacros.IsValid` _widgetdeavisoactual
    (:`Is Valid`
      (`Widget.RemoveFromParent` _widgetdeavisoactual))
    (:`Is Not Valid`
      _))
  (bind _returnvalue (`|CreateWidget` "/Game/UI/WBP_GameNotice.WBP_GameNotice_C"))
  (`/Game/UI/WBP_GameNotice.SetNoticeMessage` _returnvalue "¡DERROTA!")
  (`UserWidget.AddToViewport` _returnvalue 0)
  (set `self.WidgetDeAvisoActual` _returnvalue))

(event `self.OnReceiveOtherPlayerNoticeUI`
  (params (OtherPlayerName :type String))
  (bind _asbp_dc_pawn (cast `/Game/Blueprints/BP_DC_Pawn` (`Controller.K2_GetPawn` (`GameplayStatics.GetPlayerController` 0))))
  (bind _widgetdeavisoactual (`/Game/Blueprints/BP_DC_Pawn.WidgetDeAvisoActual` _asbp_dc_pawn))
  (`/Engine/EditorBlueprintResources/StandardMacros.IsValid` _widgetdeavisoactual
    (:`Is Valid`
      (`Widget.RemoveFromParent` _widgetdeavisoactual))
    (:`Is Not Valid`
      _))
  (bind _returnvalue (`|CreateWidget` "/Game/UI/WBP_GameNotice.WBP_GameNotice_C"))
  (`/Game/UI/WBP_GameNotice.SetNoticeMessage` _returnvalue (`KismetStringLibrary.Concat_StrStr` OtherPlayerName "\" ha sido eliminado\""))
  (`UserWidget.AddToViewport` _returnvalue 0)
  (set `/Game/Blueprints/BP_DC_Pawn.WidgetDeAvisoActual` _returnvalue _asbp_dc_pawn))

(event `self.OnReceiveScoreboardUI`
  (bind _returnvalue (`|CreateWidget` "/Game/UI/WBP_Scoreboard.WBP_Scoreboard_C"))
  (`UserWidget.AddToViewport` _returnvalue 0))

(fn `UserConstructionScript`)